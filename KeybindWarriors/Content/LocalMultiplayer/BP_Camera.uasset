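; BP_Camera is a shared-view camera actor for local multiplayer that also handles spawning for two players.
; On BeginPlay it shuffles the BP_Spawnpoints actors, creates any missing local player, then spawns and possesses a TopDownCharacter at a random, distinct spawnpoint for each.
; It then loops over all TopDownCharacters and sets itself as the view target of each matching player controller.
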(event EventBeginPlay
  (bind _outactors (Actor|GetAllActorsOfClass "/Game/LocalMultiplayer/BP_Spawnpoints.BP_Spawnpoints_C"))
  (bind _output_get (Variables|Default|SetSpawnpointReference _outactors))
  (Utilities|Array|Shuffle _output_get)
  (for _index (range 0 1)
    (bind _output_get_2 (Variables|Default|SetSpawnpointIndex _index))
    (Utilities|IsValid (Game|GetPlayerController _output_get_2)
      (:Is%20Valid
        _)
      (:Is%20Not%20Valid
        (Class|GameplayStatics|CreatePlayer (Variables|Default|GetSpawnpointIndex))))
    (bind _returnvalue (Game|SpawnActorfromClass "/Game/TopDownBP/Blueprints/TopDownCharacter.TopDownCharacter_C" (Transformation|GetActorTransform (Utilities|Array|Get(acopy) (Variables|Default|GetSpawnpointReference) (Variables|Default|GetSpawnpointIndex))) "Undefined" 0 0))
    (Pawn|Possess (Game|GetPlayerController (Variables|Default|GetSpawnpointIndex)) _returnvalue)
    (Development|PrintString "Hello"))
  (bind _outactors_2 (Actor|GetAllActorsOfClass "/Game/TopDownBP/Blueprints/TopDownCharacter.TopDownCharacter_C"))
  (for (_ _array_index) _outactors_2
    (Utilities|IsValid (Game|GetPlayerController _array_index)
      (:Is%20Valid
        (Game|Player|SetViewTargetwithBlend (Game|GetPlayerController _array_index) self 0.0 "VTBlend_Linear" 0.0 false)))))

(fn ConstructionScript)