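; Death circle that shrinks over time and ends the run of a grid movement character that leaves it.
; After a ten-second delay following BeginPlay, a gate opens and Tick reduces the static mesh's X and Y world scale by a fixed, frame-rate-dependent step.
; When a BP_GridMovementCharacter stops overlapping the Sphere, it calls Finish on that character and closes the gate, halting the shrink.
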(event OnComponentEndOverlap(Sphere)
  (params (OverlappedComponent :type Primitive%20Component%20Object%20Reference) (OtherActor :type Actor%20Object%20Reference) (OtherComp :type Primitive%20Component%20Object%20Reference) (OtherBodyIndex :type Integer))
  (bind _asbp_grid_movement_character (Utilities|Casting|CastToBP_GridMovementCharacter OtherActor))
  (Default|Finish _asbp_grid_movement_character)
  (Utilities|FlowControl|Gate true) ; enters at Close
)

(event EventBeginPlay
  (Variables|Default|SetCurrentScale (Transformation|GetWorldScale (Variables|Default|GetStaticMesh)))
  (Utilities|FlowControl|Delay 1e+01)
  (Utilities|FlowControl|Gate true) ; enters at Open
)

(event EventTick
  (params (DeltaSeconds :type Float%20%28single-precision%29))
  (Utilities|FlowControl|Gate true
    (:Exit
      (bind _output_get (Variables|Default|SetCurrentScale (Math|Vector|MakeVector (- (.x (Variables|Default|GetCurrentScale)) 0.001) (- (.y (Variables|Default|GetCurrentScale)) 0.001) (.z (Variables|Default|GetCurrentScale)))))
      (Transformation|SetWorldScale3D (Variables|Default|GetStaticMesh) _output_get))))

(fn ConstructionScript)