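; Actor component that fades a static mesh actor out and back in when its hidden state is toggled.
; BeginPlay caches the owner's materials and creates a dynamic instance of a fade material.
; ToggleHideMesh swaps every slot to that instance when hiding.
; Tick drives its Fade parameter through a curve at a set rate, restoring the original materials once fully visible.
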(event EventBeginPlay
  (bind _asstatic_mesh_actor (Utilities|Casting|CastToStaticMeshActor (Components|GetOwner)))
  (bind _output_get (Variables|Default|SetParentMesh _asstatic_mesh_actor))
  (Variables|Default|SetBaseMaterials (Rendering|Material|GetMaterials (Variables|/Script/Engine.StaticMeshActor|GetStaticMeshComponent _output_get)))
  (bind _returnvalue (Rendering|Material|CreateDynamicMaterialInstance (Variables|Default|GetFadeMaterial) "None" :!class /Script/Engine.KismetMaterialLibrary))
  (Variables|Default|SetFadeMaterialMID _returnvalue))

(event EventTick
  (params (DeltaSeconds :type Float%20%28single-precision%29))
  (if (Variables|Default|GetHidden)
    (Variables|Default|SetCurrentFade (Math|Float|Clamp(Float) (- (Variables|Default|GetCurrentFade) (* (Utilities|Time|GetWorldDeltaSeconds) (Variables|Default|GetFadeRate)))))
    (else
      (Variables|Default|SetCurrentFade (Math|Float|Clamp(Float) (+ (Variables|Default|GetCurrentFade) (* (Utilities|Time|GetWorldDeltaSeconds) (Variables|Default|GetFadeRate)))))))
  (Rendering|Material|SetScalarParameterValue (Variables|Default|GetFadeMaterialMID) "Fade" (Math|Curves|GetFloatValue (Variables|Default|GetFadeCurve) (Variables|Default|GetCurrentFade)) :!class /Script/Engine.MaterialInstanceDynamic)
  (if (and (== (Variables|Default|GetCurrentFade) 1.0) (not (Variables|Default|GetHidden)))
    (for (_array_element _array_index) (Variables|Default|GetBaseMaterials)
      (Rendering|Material|SetMaterial (Variables|/Script/Engine.StaticMeshActor|GetStaticMeshComponent (Variables|Default|GetParentMesh)) _array_index _array_element))))

(fn ToggleHideMesh
  (params (Hidden :type Boolean))
  (bind _parentmesh (Variables|Default|GetParentMesh))
  (bind _staticmeshcomponent (Variables|/Script/Engine.StaticMeshActor|GetStaticMeshComponent _parentmesh))
  (if (Math|Boolean|NotEqual(Boolean) Hidden (Variables|Default|GetHidden))
    (bind _output_get (Variables|Default|SetHidden Hidden))
    (if _output_get
      (for (_ _array_index) (Rendering|Material|GetMaterials _staticmeshcomponent)
        (Rendering|Material|SetMaterial _staticmeshcomponent _array_index (Variables|Default|GetFadeMaterialMID))))))