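; BP_Camera is a shared camera that keeps two players in view.
; On BeginPlay it caches the pawns of player indices 0 and 1 and becomes the view target of the first player controller.
; Each Tick it moves to the midpoint between both pawns and smoothly interpolates the spring arm length according to their distance, zooming out as they separate.
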(event EventBeginPlay
  (Variables|Default|SetPlayer1Char (Game|Player|GetPlayerPawn 0))
  (Variables|Default|SetPlayer2Char (Game|Player|GetPlayerPawn 1))
  (Game|Player|SetViewTargetwithBlend (Game|GetPlayerController 0) self 0.0 "VTBlend_Linear" 0.0 false))

(event EventTick
  (params (DeltaSeconds :type Float%20%28single-precision%29))
  (bind _player1char (Variables|Default|GetPlayer1Char))
  (bind _player2char (Variables|Default|GetPlayer2Char))
  (Transformation|SetActorLocation (/ (+ (Transformation|GetActorLocation _player1char) (Transformation|GetActorLocation _player2char)) 2.0) false false)
  (Variables|/Script/Engine.SpringArmComponent|SetTargetArmLength (Variables|Default|GetSpringArm) (Math|Interpolation|FInterpTo (Variables|/Script/Engine.SpringArmComponent|GetTargetArmLength (Variables|Default|GetSpringArm)) (Math|Float|Lerp 1.4e+03 5e+03 (/ (Transformation|GetDistanceTo _player1char _player2char) 4e+03)) (Utilities|Time|GetWorldDeltaSeconds) 3.0)))

(fn ConstructionScript)