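; BP_GridTile is a grid tile bound to a gamepad face button, which sets the color and rotation of its arrow indicator.
; On BeginPlay it derives the button index, and tiles tagged as player spawns create, possess and tint that player's BP_GridMovementCharacter, creating local player two if needed.
; Activate shows a full-size arrow and ActivateFar a smaller, translucent one.
; Deactivate hides it unless the other player's near-tile lists contain this tile.
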(event EventBeginPlay
  (bind _returnvalue (Transformation|GetActorLocation))
  (bind _keytopress (Variables|Default|GetKeytoPress))
  (bind _returnvalue_2 (+ _returnvalue "0, 0,200.000000"))
  (if (== _keytopress "Gamepad_FaceButton_Bottom")
    (Variables|Default|SetIndex 0)
    (if (Actor|ActorHasTag "Player1Spawn") :!label _label
      (bind _returnvalue_3 (Game|SpawnActorfromClass "/Game/TopDownBP/Character/BP_GridMovementCharacter.BP_GridMovementCharacter_C" (Math|Transform|MakeTransform _returnvalue_2 "0, 0, 0" "1,1,1") "Undefined" 0 0))
      (Variables|/Game/TopDownBP/Character/BP_GridMovementCharacter.BP_GridMovementCharacter_C|SetControllerID _returnvalue_3 0)
      (Pawn|Possess (Game|GetPlayerController 0) _returnvalue_3)
      (bind _output_get (Variables|/Game/TopDownBP/Character/BP_GridMovementCharacter.BP_GridMovementCharacter_C|SetCurrentTile _returnvalue_3 self))
      (Variables|/Game/TopDownBP/Character/BP_GridMovementCharacter.BP_GridMovementCharacter_C|SetPreviousTile _returnvalue_3 _output_get)
      (Default|Initialize _returnvalue_3)
      (Rendering|Material|SetVectorParameterValueonMaterials (Variables|/Game/TopDownBP/Character/BP_GridMovementCharacter.BP_GridMovementCharacter_C|GetSphere _returnvalue_3) "GoblinColor" (Math|Conversions|ToVector(LinearColor) "(R=1.000000,G=0.030725,B=0.020778,A=1.000000)"))
      (elif (Actor|ActorHasTag "Player2Spawn")
        (bind _returnvalue_4 (Class|GameplayStatics|CreatePlayer 1))
        (bind _returnvalue_5 (Game|SpawnActorfromClass "/Game/TopDownBP/Character/BP_GridMovementCharacter.BP_GridMovementCharacter_C" (Math|Transform|MakeTransform _returnvalue_2 "0, 0, 0" "1,1,1") "Undefined" 0 0))
        (Variables|/Game/TopDownBP/Character/BP_GridMovementCharacter.BP_GridMovementCharacter_C|SetControllerID _returnvalue_5 1)
        (Pawn|Possess _returnvalue_4 _returnvalue_5)
        (bind _output_get_2 (Variables|/Game/TopDownBP/Character/BP_GridMovementCharacter.BP_GridMovementCharacter_C|SetCurrentTile _returnvalue_5 self))
        (Variables|/Game/TopDownBP/Character/BP_GridMovementCharacter.BP_GridMovementCharacter_C|SetPreviousTile _returnvalue_5 _output_get_2)
        (Default|Initialize _returnvalue_5)
        (Rendering|Material|SetVectorParameterValueonMaterials (Variables|/Game/TopDownBP/Character/BP_GridMovementCharacter.BP_GridMovementCharacter_C|GetSphere _returnvalue_5) "GoblinColor" (Math|Conversions|ToVector(LinearColor) "(R=0.000000,G=0.067954,B=1.000000,A=1.000000)"))))
    (elif (== _keytopress "Gamepad_FaceButton_Left")
      (Variables|Default|SetIndex 1)
      (goto _label)
      (elif (== _keytopress "Gamepad_FaceButton_Top")
        (Variables|Default|SetIndex 2)
        (goto _label)
        (elif (== _keytopress "Gamepad_FaceButton_Right")
          (Variables|Default|SetIndex 3)
          (goto _label))))))

(fn ConstructionScript
  (Components|StaticMesh|SetStaticMesh (Variables|Default|GetStaticMesh) (Variables|Default|GetVisibleMesh)))

(fn Activate
  (bind _arrowindication (Variables|Default|GetArrowIndication))
  (Transformation|SetWorldScale3D _arrowindication "1.000000,1.000000,1.000000")
  (Rendering|SetVisibility _arrowindication true false)
  (Rendering|Material|SetVectorParameterValueonMaterials _arrowindication "Color" (Math|Conversions|ToVector(LinearColor) (Utilities|Select :Index (Variables|Default|GetIndex) :Option%200 "(R=0.000000,G=0.442708,B=0.035681,A=1.000000)" :Option%201 "(R=0.000000,G=0.076369,B=1.000000,A=1.000000)" :Option%202 "(R=0.458333,G=0.394887,B=0.000000,A=1.000000)" :Option%203 "(R=0.656250,G=0.000000,B=0.015861,A=1.000000)")))
  (Transformation|SetRelativeRotation _arrowindication (Utilities|Select :Index (Variables|Default|GetIndex) :Option%200 "0,-90.000000, 0" :Option%201 "0, 0, 0" :Option%202 "0.000000,90.000000,0.000000" :Option%203 "0.000000,180.000000,0.000000") false false)
  (return))

(fn Deactivate
  (params (PlayerIndex :type Integer))
  (bind _self self)
  (bind _asbp_grid_movement_character (Utilities|Casting|CastToBP_GridMovementCharacter (Game|Player|GetPlayerPawn (Utilities|Select :Index PlayerIndex :Option%200 1 :Option%201 0))))
  (if (not (or (Utilities|Array|ContainsItem (Variables|/Game/TopDownBP/Character/BP_GridMovementCharacter.BP_GridMovementCharacter_C|GetKindaNearTiles _asbp_grid_movement_character) _self) (Utilities|Array|ContainsItem (Variables|/Game/TopDownBP/Character/BP_GridMovementCharacter.BP_GridMovementCharacter_C|GetNearTiles _asbp_grid_movement_character) _self)))
    (Rendering|SetVisibility (Variables|Default|GetArrowIndication) false false)
    (return)))

(fn ActivateFar
  (bind _arrowindication (Variables|Default|GetArrowIndication))
  (Transformation|SetWorldScale3D _arrowindication "0.700000,0.700000,0.700000")
  (Rendering|SetVisibility _arrowindication true false)
  (Rendering|Material|SetVectorParameterValueonMaterials _arrowindication "Color" (Math|Conversions|ToVector(LinearColor) (Utilities|Select :Index (Variables|Default|GetIndex) :Option%200 "(R=0.000000,G=0.442708,B=0.035681,A=0.500000)" :Option%201 "(R=0.000000,G=0.076369,B=1.000000,A=0.500000)" :Option%202 "(R=0.458333,G=0.394887,B=0.000000,A=0.500000)" :Option%203 "(R=0.656250,G=0.000000,B=0.015861,A=0.500000)")))
  (Transformation|SetRelativeRotation _arrowindication (Utilities|Select :Index (Variables|Default|GetIndex) :Option%200 "0,-90.000000, 0" :Option%201 "0, 0, 0" :Option%202 "0.000000,90.000000,0.000000" :Option%203 "0.000000,180.000000,0.000000") false false)
  (return))