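; AC_Canon is a cannon actor that fires when a BP_GridMovementCharacter overlaps it.
; It spawns an AC_CannonBall at its Arrow, passing a scaled forward vector, with an explosion effect and 2D sound.
; Chained MoveComponentTo calls tilt the Cannon component and ease it back, with CanShoot blocking another shot until the motion finishes.
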(event Collision|EventActorBeginOverlap
  (params (OtherActor :type Actor%20Object%20Reference))
  (bind _arrow (Variables|Default|GetArrow))
  (bind _returnvalue (Transformation|GetWorldLocation _arrow))
  (if (Variables|Default|GetCanShoot?)
    (Utilities|Casting|CastToBP_GridMovementCharacter OtherActor)
    (Game|SpawnActorfromClass "/Game/Canon/AC_CannonBall.AC_CannonBall_C" (Math|Transform|MakeTransform _returnvalue "0, 0, 0" "1,1,1") "Undefined" 0 (* (Math|Vector|GetForwardVector _arrow) 15) 0)
    (Effects|SpawnEmitteratLocation "/Game/Canon/VFX_GrenadeEXP_air.VFX_GrenadeEXP_air" _returnvalue)
    (Audio|SpawnSound2D "/Game/Canon/Explosion01.Explosion01" 1.0 1.0 0.0 0)
    (Variables|Default|SetCanShoot? false)
    (Components|MoveComponentTo (Variables|Default|GetCannon) "0, 0, 0" "0, 0,-30.000000" false false 0.2 false)
    (Components|MoveComponentTo (Variables|Default|GetCannon) "0, 0, 0" "0, 0, 0" false true 0.75 false)
    (Variables|Default|SetCanShoot? true)))

(fn ConstructionScript)